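; BP_PuzzleIvan is a placement puzzle pairing seven child-actor pressure triggers (BP_Pressionadores) with seven pieces from the Pecas array.
; On BeginPlay it registers each trigger in Sinais, assigns its specific piece and sets it to accept a single BP_PecasIvan occupant at its box.
; It also gives each piece its own mesh by index, then runs the parent BeginPlay.
; Sinalizar forwards only true signals to the Receptor.
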(event `self.ReceiveBeginPlay`
  (for (_array_element _array_index) (`|MakeArray` (`ChildActorComponent.ChildActor` (`self.BP_Pressionadores0`)) (`ChildActorComponent.ChildActor` (`self.BP_Pressionadores1`)) (`ChildActorComponent.ChildActor` (`self.BP_Pressionadores2`)) (`ChildActorComponent.ChildActor` (`self.BP_Pressionadores3`)) (`ChildActorComponent.ChildActor` (`self.BP_Pressionadores4`)) (`ChildActorComponent.ChildActor` (`self.BP_Pressionadores5`)) (`ChildActorComponent.ChildActor` (`self.BP_Pressionadores6`)))
    (bind _asbp_pressionadores (cast `/Game/BP_Objetos/Classes_Abstratas/BP_Pressionadores` _array_element))
    (`KismetArrayLibrary.Array_Add` (`self.Sinais`) _asbp_pressionadores)
    (set `/Game/BP_Objetos/Classes_Abstratas/BP_Pressionadores.Objeto Especifico` (`|GetArrayItem` (`self.Pecas`) _array_index) _asbp_pressionadores)
    (`/Game/BP_Objetos/Classes_Abstratas/BP_Pressionadores.SetarParaUmOcupante` _asbp_pressionadores (`SceneComponent.K2_GetComponentToWorld` (`/Game/BP_Objetos/Classes_Abstratas/BP_Pressionadores.Box` _asbp_pressionadores)) "/Game/BP_Objetos/BP_PecasIvan.BP_PecasIvan_C"))
  (for (_array_element_2 _array_index_2) (`self.Pecas`)
    (`StaticMeshComponent.SetStaticMesh` (`/Game/BP_Objetos/Classes_Abstratas/BP_ObjetoInterajivel.Mesh` _array_element_2) (select `int` _array_index_2 :`0` "/Game/ModelosProprios/Objetos/Puzzle_Ivan/Peca0.Peca0" :`1` "/Game/ModelosProprios/Objetos/Puzzle_Ivan/Peca1.Peca1" :`2` "/Game/ModelosProprios/Objetos/Puzzle_Ivan/Peca2.Peca2" :`3` "/Game/ModelosProprios/Objetos/Puzzle_Ivan/Peca3.Peca3" :`4` "/Game/ModelosProprios/Objetos/Puzzle_Ivan/Peca4.Peca4" :`5` "/Game/ModelosProprios/Objetos/Puzzle_Ivan/Peca5.Peca5" :`6` "/Game/ModelosProprios/Objetos/Puzzle_Ivan/Peca6.Peca6" :!type "StaticMesh Object Reference")))
  (`parent.ReceiveBeginPlay`))

(event `self.Sinalizar`
  (params (Sinal :type Boolean))
  (if Sinal
    (`self.Sinalizar` (`self.Receptor`) Sinal)))

(fn `UserConstructionScript`
  (`parent.UserConstructionScript`))