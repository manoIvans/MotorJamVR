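; BP_Bau is a chest that opens once, when a BP_Chave key enters its sphere.
; On overlap it spawns a bottle and a star-meshed BP_Caixinha with physics off, flags itself open and calls MudarSinal.
; It snaps the key to a spawn point and triggers its Abrir.
; A per-tick wait loop holds the chest animation and sound until the key is no longer valid.
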(event `self.Sphere.OnComponentBeginOverlap`
  (params (OverlappedComponent :type "PrimitiveComponent Object Reference") (OtherActor :type "Actor Object Reference") (OtherComp :type "PrimitiveComponent Object Reference") (OtherBodyIndex :type Integer) (bFromSweep :type Boolean) (SweepResult :type "HitResult Structure (by ref)"))
  (bind _skeletalmesh (`self.SkeletalMesh`))
  (if (not (`self.Aberto`))
    (if (== (`GameplayStatics.GetObjectClass` OtherActor) "/Game/BP_Objetos/BP_Chave.BP_Chave_C")
      (bind _asbp_chave (cast `/Game/BP_Objetos/BP_Chave` OtherActor))
      (`SkeletalMeshComponent.SetAllBodiesBelowPhysicsDisabled` _skeletalmesh (`SkinnedMeshComponent.GetBoneName` _skeletalmesh 1) true true)
      (`self.SpawnarObjetos`)
      (bind _output_get (set `self.Aberto` true))
      (`self.MudarSinal` _output_get)
      (`self.K2_SetActorTransform` _asbp_chave (`SceneComponent.K2_GetComponentToWorld` (`self.ChaveSpawn`)) false true)
      (`/Game/BP_Objetos/BP_Chave.Abrir` _asbp_chave)
      (`/Engine/EditorBlueprintResources/StandardMacros.IsValid` _asbp_chave :!label _label
        (:`Is Valid`
          (`KismetSystemLibrary.DelayUntilNextTick`)
          (goto _label))
        (:`Is Not Valid`
          (`SkeletalMeshComponent.PlayAnimation` (`self.SkeletalMesh`) "/Game/ModelosProprios/Aqui/Bau/bauzao_Anim.bauzao_Anim" false)
          (`AudioComponent.Play` (`self.Som`) 0.0))))))

(fn `SpawnarObjetos`
  (bind (_returnvalue_location _returnvalue_rotation) (`KismetMathLibrary.BreakTransform` (`SceneComponent.K2_GetComponentToWorld` (`self.GarrafaSpawn`))))
  (bind _returnvalue (`|SpawnActorFromClass` "/Game/BP_Objetos/BP_Garrafa.BP_Garrafa_C" (`KismetMathLibrary.MakeTransform` _returnvalue_location _returnvalue_rotation) "AlwaysSpawn" "MultiplyWithRoot" null null))
  (`PrimitiveComponent.SetSimulatePhysics` (`/Game/BP_Objetos/BP_Garrafa.StaticMesh` _returnvalue) false)
  (bind _returnvalue_2 (`|SpawnActorFromClass` "/Game/BP_Objetos/BP_Caixinha.BP_Caixinha_C" (`SceneComponent.K2_GetComponentToWorld` (`self.CaixinhaSpawn`)) "Undefined" "MultiplyWithRoot" null null))
  (bind _caixamesh (`/Game/BP_Objetos/BP_Caixinha.CaixaMesh` _returnvalue_2))
  (`PrimitiveComponent.SetSimulatePhysics` _caixamesh false)
  (`StaticMeshComponent.SetStaticMesh` _caixamesh "/Game/ModelosProprios/Aqui/estrela.estrela"))

(fn `UserConstructionScript`)