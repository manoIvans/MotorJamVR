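; BP_Receptor is a base receiver actor that switches on only when all of its linked signals (Sinais) are active.
; On BeginPlay it binds to each signal's Atualizou update event and runs an initial evaluation.
; AtualizarSinais ANDs every Ativo flag into Ativado, then passes the result to Sinalizar, an empty event for child classes to implement.
; An empty signal list counts as activated.
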(event `self.ReceiveBeginPlay`
  (for _array_element (`self.Sinais`)
    (add `/Game/BP_Objetos/Classes_Abstratas/BP_Ativadores.Atualizou` _array_element (delegate `AtualizarSinais`)))
  (`self.AtualizarSinais`))

(event `AtualizarSinais`
  (set `self.Ativado` true)
  (for _array_element (`self.Sinais`)
    (if (not (`/Game/BP_Objetos/Classes_Abstratas/BP_Ativadores.Ativo` _array_element))
      (set `self.Ativado` false)
      (break)))
  (`self.Sinalizar` (`self.Ativado`)))

(event `Sinalizar`
  (params (Sinal :type Boolean)))

(fn `UserConstructionScript`)