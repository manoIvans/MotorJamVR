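; Dungeon double-door actor that swings open once when its Sinalizar event receives a true signal.
; The Aberto flag blocks retriggering, and a creaking sound plays with slightly randomized pitch.
; A Delay-driven loop rotates both leaves in opposite yaw steps until the left one reaches its limit, with no Timeline and no closing logic.
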(event `self.Sinalizar`
  (params (Sinal :type Boolean))
  (bind _sm_doorway_large_door_right (`self.SM_DoorWay_Large_Door_Right`))
  (bind _sm_doorway_large_door_left (`self.SM_DoorWay_Large_Door_Left`))
  (bind _returnvalue (`SceneComponent.GetRelativeTransform` _sm_doorway_large_door_left))
  (bind _returnvalue_2 (`SceneComponent.GetRelativeTransform` _sm_doorway_large_door_right))
  (bind _returnvalue_location (`KismetMathLibrary.BreakTransform` (`SceneComponent.K2_GetComponentToWorld` (`self.DefaultSceneRoot`))))
  (if (and Sinal (not (`self.aberto`)))
    (set `self.aberto` true)
    (`GameplayStatics.PlaySoundAtLocation` "/Game/BP_Objetos/Sons/wooden-door-creaking-102413.wooden-door-creaking-102413" _returnvalue_location (struct) 1.0 (`KismetMathLibrary.RandomFloatInRange` 0.97 1.02) 0.0 null null null null)
    (if (not (>= (.yaw (.rotation (`SceneComponent.GetRelativeTransform` (`self.SM_DoorWay_Large_Door_Left`)))) 70.0)) :!label _label
      (`SceneComponent.K2_SetRelativeTransform` _sm_doorway_large_door_right (`KismetMathLibrary.MakeTransform` (.location _returnvalue_2) (`KismetMathLibrary.MakeRotator` (.roll (.rotation _returnvalue_2)) (.pitch (.rotation _returnvalue_2)) (+ -0.5 (.yaw (.rotation _returnvalue_2))))) false false)
      (`SceneComponent.K2_SetRelativeTransform` _sm_doorway_large_door_left (`KismetMathLibrary.MakeTransform` (.location _returnvalue) (`KismetMathLibrary.MakeRotator` (.roll (.rotation _returnvalue)) (.pitch (.rotation _returnvalue)) (+ 0.5 (.yaw (.rotation _returnvalue)))) (.scale _returnvalue)) false false)
      (`KismetSystemLibrary.Delay` 0.01)
      (goto _label))))

(fn `UserConstructionScript`)