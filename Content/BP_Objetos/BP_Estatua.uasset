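; BP_Estatua is a statue that acts as a socket for a BP_Garrafa bottle and sets a signal once filled.
; When a bottle overlaps its Box, it retries releasing the bottle's grab component every tick until it succeeds.
; It then disables and destroys that component, calls Sonzinhoyip, stops physics and snaps the bottle mesh to GarrafaPos, keeping its scale.
; Finally it calls MudarSinal(true).
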(event `self.ReceiveBeginPlay`
  (`parent.ReceiveBeginPlay`))

(event `self.Box.OnComponentBeginOverlap`
  (params (OverlappedComponent :type "PrimitiveComponent Object Reference") (OtherActor :type "Actor Object Reference") (OtherComp :type "PrimitiveComponent Object Reference") (OtherBodyIndex :type Integer) (bFromSweep :type Boolean) (SweepResult :type "HitResult Structure (by ref)"))
  (bind (_returnvalue_location _returnvalue_rotation) (`KismetMathLibrary.BreakTransform` (`SceneComponent.K2_GetComponentToWorld` (`self.GarrafaPos`))))
  (if (== (`GameplayStatics.GetObjectClass` OtherActor) "/Game/BP_Objetos/BP_Garrafa.BP_Garrafa_C")
    (bind _asbp_garrafa (cast `/Game/BP_Objetos/BP_Garrafa` OtherActor))
    (bind _grabcomponent (`/Game/BP_Objetos/BP_Garrafa.GrabComponent` _asbp_garrafa))
    (bind _breleased (`/Game/VRTemplate/Blueprints/GrabComponent.TryRelease` _grabcomponent :!label _label))
    (if _breleased
      (set `/Game/VRTemplate/Blueprints/GrabComponent.GrabType` "NewEnumerator0" _grabcomponent)
      (`ActorComponent.K2_DestroyComponent` _grabcomponent)
      (`/Game/BP_Objetos/BP_Garrafa.Sonzinhoyip` _asbp_garrafa)
      (bind _mesh (`/Game/BP_Objetos/Classes_Abstratas/BP_ObjetoInterajivel.Mesh` _asbp_garrafa))
      (`PrimitiveComponent.SetSimulatePhysics` _mesh false)
      (`PrimitiveComponent.SetPhysicsLinearVelocity` _mesh (0.0 0.0 0.0) false "None")
      (`SceneComponent.K2_SetWorldTransform` _mesh (`KismetMathLibrary.MakeTransform` _returnvalue_location _returnvalue_rotation (`self.GetActorScale3D` _asbp_garrafa)) false false)
      (`self.MudarSinal` true)
      (else
        (`KismetSystemLibrary.DelayUntilNextTick`)
        (goto _label)))))

(fn `UserConstructionScript`
  (`parent.UserConstructionScript`))