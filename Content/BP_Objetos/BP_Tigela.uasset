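; BP_Tigela is a bowl socket that holds one BP_Caixinha and passes a true signal to its parent only when that occupant is ObjetoEspecifico.
; The inherited Detectou event drops an occupant that left the Box and adopts the first overlapping caixinha.
; A DelayUntilNextTick loop, used instead of Tick, snaps the occupant to the Arrow whenever it is not held, zeroing velocity and disabling physics.
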(event `self.ReceiveBeginPlay`
  (`parent.ReceiveBeginPlay`)
  (add `self.Detectou` (delegate `Detectou_Event`)))

(event `Detectou_Event`
  (bind _ocupante (`self.ocupante`))
  (bind _overlappingactors (`PrimitiveComponent.GetOverlappingActors` (`self.Box`) "/Game/BP_Objetos/BP_Caixinha.BP_Caixinha_C"))
  (`/Engine/EditorBlueprintResources/StandardMacros.IsValid` _ocupante
    (:`Is Valid`
      (if (not (`KismetArrayLibrary.Array_Contains` _overlappingactors _ocupante))
        (set `self.ocupante` null)
        (if (> (`KismetArrayLibrary.Array_Length` _overlappingactors) 0)
          (bind _asbp_caixinha (cast `/Game/BP_Objetos/BP_Caixinha` (`|GetArrayItem` _overlappingactors) :!label _label))
          (bind _output_get (set `self.ocupante` _asbp_caixinha))
          (if true :!label _label_2
            (`self.PosicionarObjetoCorretamente` _output_get)
            (`KismetSystemLibrary.DelayUntilNextTick`)
            (goto _label_2)))))
    (:`Is Not Valid`
      (goto _label))))

(fn `MudarSinal`
  (params (Sinal :type Boolean))
  (`parent.MudarSinal` (and Sinal (== (`self.ocupante`) (`self.Objeto Especifico`)))))

(fn `PosicionarObjetoCorretamente`
  (params (Objeto :type "/Game/BP_Objetos/BP_Caixinha Object Reference"))
  (bind _caixamesh (`/Game/BP_Objetos/BP_Caixinha.CaixaMesh` Objeto))
  (bind (_returnvalue_location _returnvalue_rotation) (`KismetMathLibrary.BreakTransform` (`SceneComponent.K2_GetComponentToWorld` (`self.Arrow`))))
  (`/Engine/EditorBlueprintResources/StandardMacros.IsValid` Objeto
    (:`Is Valid`
      (if (not (`/Game/VRTemplate/Blueprints/GrabComponent.bIsHeld` (`/Game/BP_Objetos/BP_Caixinha.GrabComponent` Objeto)))
        (`self.K2_SetActorTransform` Objeto (`KismetMathLibrary.MakeTransform` _returnvalue_location _returnvalue_rotation (`self.GetActorScale3D` Objeto)) false false)
        (`PrimitiveComponent.SetPhysicsLinearVelocity` _caixamesh (0.0 0.0 0.0) false "None")
        (`PrimitiveComponent.SetSimulatePhysics` _caixamesh false))
      (return))))

(fn `UserConstructionScript`
  (`parent.UserConstructionScript`))