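; Base class for pressure-triggered objects (Pressionadores) that switch an Ativo signal according to what overlaps their Box.
; Each begin or end overlap re-runs DetectarPressao, fires the Detectou dispatcher and passes the result to MudarSinal.
; DetectarPressao looks only for ObjetoEspecifico when it is valid, otherwise any actor other than itself counts.
; MudarSinal updates Ativo, fires Atualizou and prints a debug string only when the state changes.
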(event `self.ReceiveTick`
  (params (DeltaSeconds :type "Float (single-precision)"))
  (`parent.ReceiveTick` DeltaSeconds))

(event `self.Box.OnComponentBeginOverlap`
  (params (OverlappedComponent :type "PrimitiveComponent Object Reference") (OtherActor :type "Actor Object Reference") (OtherComp :type "PrimitiveComponent Object Reference") (OtherBodyIndex :type Integer) (bFromSweep :type Boolean) (SweepResult :type "HitResult Structure (by ref)"))
  (bind _esta_pressionado (`self.DetectarPressao` (`self.Objeto Especifico`) :!label _label))
  (`self.Detectou`)
  (`self.MudarSinal` _esta_pressionado))

(event `self.Box.OnComponentEndOverlap`
  (params (OverlappedComponent :type "PrimitiveComponent Object Reference") (OtherActor :type "Actor Object Reference") (OtherComp :type "PrimitiveComponent Object Reference") (OtherBodyIndex :type Integer))
  (goto _label))

(fn `DetectarPressao`
  (params (ObjetoEspecifico :type "Actor Object Reference"))
  (returns (`Esta Pressionado` :type Boolean))
  (locals (Pressionado :type Boolean))
  (bind _overlappingactors (`PrimitiveComponent.GetOverlappingActors` (`self.Box`) null))
  (`/Engine/EditorBlueprintResources/StandardMacros.IsValid` ObjetoEspecifico
    (:`Is Valid`
      (set `local.Pressionado` (`KismetArrayLibrary.Array_Contains` _overlappingactors ObjetoEspecifico)))
    (:`Is Not Valid`
      (for _array_element _overlappingactors
        (if (!= _array_element self)
          (set `local.Pressionado` true)
          (return (`local.Pressionado`))))))
  (return (`local.Pressionado`)))

(fn `MudarSinal`
  (params (Sinal :type Boolean))
  (if (!= (`self.Ativo`) Sinal)
    (bind _output_get (set `self.Ativo` Sinal))
    (`self.Atualizou`)
    (`KismetSystemLibrary.PrintString` (`KismetStringLibrary.Concat_StrStr` "Setando ativo: " (`KismetStringLibrary.Conv_BoolToString` _output_get)))))

(fn `UserConstructionScript`
  (`parent.UserConstructionScript`))