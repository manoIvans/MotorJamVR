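; BP_Tigela is a bowl actor that snaps a detected BP_Caixinha box into a set pose.
; When the inherited Detectou dispatcher fires, it casts ObjetoEspecifico and loops every tick while that object overlaps its Box.
; Each pass, if the object's GrabComponent is not held, it moves the object to the Arrow's location and rotation, keeps its scale, zeroes velocity and disables physics simulation.
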(event `self.ReceiveBeginPlay`
  (`parent.ReceiveBeginPlay`)
  (add `self.Detectou` (delegate `Detectou_Event`)))

(event `Detectou_Event`
  (bind _asbp_caixinha (cast `/Game/Objetos/BP_Caixinha` (`self.Objeto Especifico`)))
  (if (`KismetArrayLibrary.Array_Contains` (`PrimitiveComponent.GetOverlappingActors` (`self.Box`) null) (`self.Objeto Especifico`)) :!label _label
    (`self.PosicionarObjetoCorretamente` _asbp_caixinha)
    (`KismetSystemLibrary.DelayUntilNextTick`)
    (goto _label)))

(fn `PosicionarObjetoCorretamente`
  (params (Objeto :type "/Game/Objetos/BP_Caixinha Object Reference"))
  (bind _caixamesh (`/Game/Objetos/BP_Caixinha.CaixaMesh` Objeto))
  (bind (_returnvalue_location _returnvalue_rotation) (`KismetMathLibrary.BreakTransform` (`SceneComponent.K2_GetComponentToWorld` (`self.Arrow`))))
  (if (not (`/Game/VRTemplate/Blueprints/GrabComponent.bIsHeld` (`/Game/Objetos/BP_Caixinha.GrabComponent` Objeto)))
    (`self.K2_SetActorTransform` Objeto (`KismetMathLibrary.MakeTransform` _returnvalue_location _returnvalue_rotation (`self.GetActorScale3D` Objeto)) false false)
    (`PrimitiveComponent.SetPhysicsLinearVelocity` _caixamesh (0.0 0.0 0.0) false "None")
    (`PrimitiveComponent.SetSimulatePhysics` _caixamesh false))
  (return))

(fn `UserConstructionScript`
  (`parent.UserConstructionScript`))